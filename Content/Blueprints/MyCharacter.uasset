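; Player Character Blueprint that handles walking, sprinting, jumping and third-person-style camera control.
; Mouse X yaws the SpringArm in world space and Mouse Y pitches it in local space, without directly rotating the actor.
; Axis inputs move the character along its own forward and right vectors.
; Space drives jump, and Left Shift switches max walk speed between walk and sprint while held.
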(event `InputAxisKey|MouseX`
  (params (AxisValue :type "Float (single-precision)"))
  (`SceneComponent.K2_AddWorldRotation` (`self.SpringArm`) (`KismetMathLibrary.MakeRotator` 0.0 0.0 AxisValue) false false))

(event `InputAxis|Forward&Back`
  (params (AxisValue :type "Float (single-precision)"))
  ;[1 1 1] Movement
  (`self.AddMovementInput` (`self.GetActorForwardVector`) AxisValue))

(event `InputAxisKey|MouseY`
  (params (AxisValue :type "Float (single-precision)"))
  (`SceneComponent.K2_AddLocalRotation` (`self.SpringArm`) (`KismetMathLibrary.MakeRotator` 0.0 AxisValue) false false))

(event `InputAxis|Right&Left`
  (params (AxisValue :type "Float (single-precision)"))
  ;[1 1 1] Movement
  (`self.AddMovementInput` (`self.GetActorRightVector`) AxisValue))

(event `Key|SpaceBar`
  (params (Key :type "Key Structure"))
  ;[1 1 1] Movement
  (:`Pressed`
    (`self.Jump`))
  (:`Released`
    (`self.StopJumping`)))

(event `Key|LeftShift`
  (params (Key :type "Key Structure"))
  (bind _charactermovement (`self.CharacterMovement`))
  (:`Pressed`
    (set `CharacterMovementComponent.MaxWalkSpeed` 600.0 _charactermovement))
  (:`Released`
    (set `CharacterMovementComponent.MaxWalkSpeed` 200.0 _charactermovement)))

(fn `UserConstructionScript`)